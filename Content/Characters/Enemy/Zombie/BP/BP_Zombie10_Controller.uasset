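; AI controller for Zombie10 that runs BT_Zombie10 when it possesses a BP_Zombie pawn.
; Perception updates for BP_Character set CanSeePlayer on the blackboard, and losing sight also records the player's current location and sets RecentlySighted.
; Walk, Run and Attack events forward to the possessed zombie, while Tick polls IsDead to stop the brain logic.
; An unconnected block for storing a home location never runs.
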(event `self.ReceiveTick`
  (params (DeltaSeconds :type "Float (single-precision)"))
  ;[1 1 1] Death
  (bind _asbp_zombie (cast `/Game/Characters/Enemy/Zombie/BP/BP_Zombie` (`self.Zombie10`)))
  (if (`/Game/Characters/Enemy/Zombie/BP/BP_Zombie.isDead?` _asbp_zombie)
    (`BrainComponent.StopLogic` (`AIController.BrainComponent` (`AIBlueprintHelperLibrary.GetAIController` self)) "Dead")))

(event `self.AIPerception.OnTargetPerceptionUpdated`
  (params (Actor :type "Actor Object Reference") (Stimulus :type "AIStimulus Structure"))
  (bind (_age _expirationage _strength _stimuluslocation _receiverlocation _tag _bsuccessfullysensed) (break `AIStimulus` Stimulus))
  (bind _returnvalue (`AIBlueprintHelperLibrary.GetBlackboard` null))
  (cast `/Game/Characters/Player/Eve/BP/BP_Character` Actor)
  (`BlackboardComponent.SetValueAsBool` _returnvalue "CanSeePlayer" _bsuccessfullysensed)
  (if (not _bsuccessfullysensed)
    (`BlackboardComponent.SetValueAsVector` _returnvalue "PlayerLocation" (`self.K2_GetActorLocation` (`GameplayStatics.GetPlayerCharacter` 0)))
    (`BlackboardComponent.SetValueAsBool` _returnvalue "RecentlySighted" true)))

(event `Walk`
  (`/Game/Characters/Enemy/Zombie/BP/BP_Zombie.Walk` (`self.Zombie10`)))

(event `Run`
  (`/Game/Characters/Enemy/Zombie/BP/BP_Zombie.Run` (`self.Zombie10`)))

(event `self.ReceivePossess`
  (params (PossessedPawn :type "Pawn Object Reference"))
  (bind _asbp_zombie (cast `/Game/Characters/Enemy/Zombie/BP/BP_Zombie` PossessedPawn))
  (set `self.Zombie10` _asbp_zombie)
  (`self.RunBehaviorTree` "/Game/Characters/Enemy/Zombie/BT_Zombie10.BT_Zombie10"))

(event `Attack`
  (`/Game/Characters/Enemy/Zombie/BP/BP_Zombie.Attack` (`self.Zombie10`)))

(fn `UserConstructionScript`)