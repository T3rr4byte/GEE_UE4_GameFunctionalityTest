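; BP_HP_Spawn_Parent is a bomb pickup actor that, despite its HP spawn name, damages the player character on contact.
; A box overlap with BP_Character passes a DoOnce and subtracts a fixed amount directly from the character's Health.
; It then activates two explosion components, toggles the mesh's visibility and destroys itself after a short delay.
; The DoOnce reset follows DestroyActor, so the bomb is effectively single-use.
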(event `self.Box.OnComponentBeginOverlap`
  (params (OverlappedComponent :type "PrimitiveComponent Object Reference") (OtherActor :type "Actor Object Reference") (OtherComp :type "PrimitiveComponent Object Reference") (OtherBodyIndex :type Integer) (bFromSweep :type Boolean) (SweepResult :type "HitResult Structure (by ref)"))
  (bind _asbp_character (cast `/Game/Characters/Player/Eve/BP/BP_Character` OtherActor))
  (`/Engine/EditorBlueprintResources/StandardMacros.DoOnce` false :!label _label
    (:`Completed`
      (set `/Game/Characters/Player/Eve/BP/BP_Character.Health` (- (`/Game/Characters/Player/Eve/BP/BP_Character.Health` _asbp_character) 45) _asbp_character)
      (`ActorComponent.Activate` (`self.Explosion02`) false)
      (`ActorComponent.Activate` (`self.P_Explosion`) false)
      (`SceneComponent.ToggleVisibility` (`self.StaticMesh`) false)
      (`KismetSystemLibrary.Delay` 3.0)
      (`self.K2_DestroyActor`)
      (goto _label :!via `Reset`))))

(fn `UserConstructionScript`)