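; BP_WoodPickup is a wood item that the player collects by walking into it, once a one-second delay after BeginPlay has passed.
; On box overlap it fills the first empty of five inventory slots on BP_Character through nested checks.
; It then destroys itself, adds an audio component and increments the character's wood count.
; With all slots full, it prints an inventory-full message and adds an audio component.
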(event `self.ReceiveBeginPlay`
  (`KismetSystemLibrary.Delay` 1.0)
  (set `self.canpickup?` true))

(event `self.Box.OnComponentBeginOverlap`
  (params (OverlappedComponent :type "PrimitiveComponent Object Reference") (OtherActor :type "Actor Object Reference") (OtherComp :type "PrimitiveComponent Object Reference") (OtherBodyIndex :type Integer) (bFromSweep :type Boolean) (SweepResult :type "HitResult Structure (by ref)"))
  (bind _returnvalue (`GameplayStatics.GetPlayerCharacter` 0))
  (if (== OtherActor _returnvalue)
    (if (`self.canpickup?`)
      (bind _asbp_character (cast `/Game/Player/Eve/BP/BP_Character` _returnvalue))
      (if (== (`/Game/Player/Eve/BP/BP_Character.Slot1_Item` _asbp_character) 0)
        (set `/Game/Player/Eve/BP/BP_Character.Slot1_Item` 1 _asbp_character)
        (`self.K2_DestroyActor` :!label _label)
        (`AddComponent|NODE_AddAudioComponent-0`)
        (bind _asbp_character_2 (cast `/Game/Player/Eve/BP/BP_Character` (`GameplayStatics.GetPlayerCharacter` 0)))
        (set `/Game/Player/Eve/BP/BP_Character.Amount_Wood` (+ (`/Game/Player/Eve/BP/BP_Character.Amount_Wood` _asbp_character_2) 1) _asbp_character_2)
        (elif (== (`/Game/Player/Eve/BP/BP_Character.Slot2_Item` _asbp_character) 0)
          (set `/Game/Player/Eve/BP/BP_Character.Slot2_Item` 1 _asbp_character)
          (goto _label)
          (elif (== (`/Game/Player/Eve/BP/BP_Character.Slot3_Item` _asbp_character) 0)
            (set `/Game/Player/Eve/BP/BP_Character.Slot3_Item` 1 _asbp_character)
            (goto _label)
            (elif (== (`/Game/Player/Eve/BP/BP_Character.Slot4_Item` _asbp_character) 0)
              (set `/Game/Player/Eve/BP/BP_Character.Slot4_Item` 1 _asbp_character)
              (goto _label)
              (elif (== (`/Game/Player/Eve/BP/BP_Character.Slot5_Item` _asbp_character) 0)
                (set `/Game/Player/Eve/BP/BP_Character.Slot5_Item` 1 _asbp_character)
                (goto _label)
                (else
                  (`KismetSystemLibrary.PrintString` "Inventory is full!")
                  (`AddComponent|NODE_AddAudioComponent-1`))))))))))

(fn `UserConstructionScript`)