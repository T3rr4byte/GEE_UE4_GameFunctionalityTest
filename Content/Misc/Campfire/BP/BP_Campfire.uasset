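; BP_Campfire is a campfire the player can light or put out with the action key while inside its sphere trigger.
; Tick polls the key; lighting spends one wood, starts fire and sound, then a delay burns it out via the shared shutoff branch.
; Overlap and toggle states are mirrored onto BP_Character.
; Without wood, a resettable DoOnce throttles the warning message and audio.
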(event `self.ReceiveTick`
  (params (DeltaSeconds :type "Float (single-precision)"))
  (bind _fire (`self.Fire`))
  ;[1 1 1] Switch fire on/off
  (bind _asbp_character (cast `/Game/Characters/Player/Eve/BP/BP_Character` (`GameplayStatics.GetPlayerCharacter` 0)))
  (if (`self.Near_Campfire?`)
    (if (`/Game/Characters/Player/Eve/BP/BP_Character.Action_Key_Pressed?` _asbp_character)
      (if (not (`self.Campfire_Active?`))
        (bind _amount_wood (`/Game/Characters/Player/Eve/BP/BP_Character.Amount_Wood` _asbp_character))
        (if (> _amount_wood 0)
          (`ActorComponent.Activate` _fire false)
          (`KismetSystemLibrary.Delay` 0.2)
          (set `self.Campfire_Active?` true)
          (`ActorComponent.Activate` (`self.campfire_sound`) false)
          (set `/Game/Characters/Player/Eve/BP/BP_Character.Campfire_State?` true _asbp_character)
          (set `/Game/Characters/Player/Eve/BP/BP_Character.Amount_Wood` (- _amount_wood 1) _asbp_character)
          ;;[1 1 1] Active time with 1 wood
          (`KismetSystemLibrary.Delay` 20.0)
          (else
            (`/Engine/EditorBlueprintResources/StandardMacros.DoOnce` false :!label _label
              (:`Completed`
                (`KismetSystemLibrary.PrintString` "Not enough wood!")
                (`AddComponent|NODE_AddAudioComponent-0`)
                (`KismetSystemLibrary.Delay` 1.5)
                (goto _label :!via `Reset`))))))
      (`ActorComponent.Deactivate` _fire)
      (`KismetSystemLibrary.Delay` 0.2)
      (set `self.Campfire_Active?` false)
      (`ActorComponent.Deactivate` (`self.campfire_sound`))
      (set `/Game/Characters/Player/Eve/BP/BP_Character.Campfire_State?` false _asbp_character))))

(event `self.Sphere.OnComponentBeginOverlap`
  (params (OverlappedComponent :type "PrimitiveComponent Object Reference") (OtherActor :type "Actor Object Reference") (OtherComp :type "PrimitiveComponent Object Reference") (OtherBodyIndex :type Integer) (bFromSweep :type Boolean) (SweepResult :type "HitResult Structure (by ref)"))
  ;[1 1 1] Switch fire on/off
  (if (== (`GameplayStatics.GetPlayerCharacter` 0) OtherActor)
    (set `self.Near_Campfire?` true)
    (set `/Game/Characters/Player/Eve/BP/BP_Character.Campfire_TPC?` true (stale `self.ReceiveTick` _asbp_character))))

(event `self.Sphere.OnComponentEndOverlap`
  (params (OverlappedComponent :type "PrimitiveComponent Object Reference") (OtherActor :type "Actor Object Reference") (OtherComp :type "PrimitiveComponent Object Reference") (OtherBodyIndex :type Integer))
  ;[1 1 1] Switch fire on/off
  (if (== (`GameplayStatics.GetPlayerCharacter` 0) OtherActor)
    (set `self.Near_Campfire?` false)
    (set `/Game/Characters/Player/Eve/BP/BP_Character.Campfire_TPC?` false (stale `self.ReceiveTick` _asbp_character))))

(fn `UserConstructionScript`)