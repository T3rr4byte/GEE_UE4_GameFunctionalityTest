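; Zombie enemy Blueprint with walk and run speeds, a melee attack, health and death.
; Attack plays a single animation with audio and opens a damage window, during which a claw-socket overlap sphere damages BP_Character, throttled by a resetting DoOnce.
; Lethal damage sets IsDead, restores Animation Blueprint mode so death can interrupt attacks, then destroys the mesh after a delay.
; Alternative collision-disable and ragdoll death logic is left unconnected.
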(event `Walk`
  ;[1 1 1] Movement
  (set `CharacterMovementComponent.MaxWalkSpeed` 30.0 (`self.CharacterMovement`)))

(event `Run`
  ;[1 1 1] Movement
  (set `CharacterMovementComponent.MaxWalkSpeed` 400.0 (`self.CharacterMovement`)))

(event `Attack`
  ;[1 1 1] Attack
  (`SkeletalMeshComponent.PlayAnimation` (`self.Mesh`) "/Game/Enemy/Zombie/Animations/Zombie10_attack.Zombie10_attack" false)
  (set `self.Attacking` true)
  (`AddComponent|NODE_AddAudioComponent-1`)
  (`KismetSystemLibrary.Delay` 2.633333)
  (if (not (`self.isDead?`))
    (set `self.Attacking` false)
    (`SkeletalMeshComponent.SetAnimationMode` (`self.Mesh`) "AnimationBlueprint")))

(event `self.Sphere.OnComponentBeginOverlap`
  (params (OverlappedComponent :type "PrimitiveComponent Object Reference") (OtherActor :type "Actor Object Reference") (OtherComp :type "PrimitiveComponent Object Reference") (OtherBodyIndex :type Integer) (bFromSweep :type Boolean) (SweepResult :type "HitResult Structure (by ref)"))
  ;[1 1 1] Deal Damage
  (if (`self.isDead?`)
    _
    (elif (`self.Attacking`)
      (bind _asbp_character (cast `/Game/Player/Eve/BP/BP_Character` OtherActor))
      (`/Engine/EditorBlueprintResources/StandardMacros.DoOnce` false :!label _label
        (:`Completed`
          (`/Game/Player/Eve/BP/BP_Character.TakeDamage` _asbp_character 11)
          (`AddComponent|NODE_AddAudioComponent-0`)
          (`KismetSystemLibrary.Delay` 2.0)
          (goto _label :!via `Reset`))))))

(event `Take_Damage`
  (params (Incoming_Damage :type Integer))
  ;[1 1 1] Health
  (if (not (`self.isDead?`))
    (bind _output_get (set `self.Health` (- (`self.Health`) Incoming_Damage)))
    (if (<= _output_get 0)
      (set `self.isDead?` true)
      (`AddComponent|NODE_AddAudioComponent-2`)
      ;[1 1 1] required to trigger death animation while within attack animation
      (`SkeletalMeshComponent.SetAnimationMode` (`self.Mesh`) "AnimationBlueprint")
      ;[1 1 1] Despawn
      (`KismetSystemLibrary.Delay` 20.0)
      (`ActorComponent.K2_DestroyComponent` (`self.Mesh`))
      (else
        (set `self.isDead?` false)))))

(fn `UserConstructionScript`
  (`SceneComponent.K2_AttachToComponent` (`self.Sphere`) (`self.Mesh`) "ClawSocket" "KeepRelative" "KeepRelative" "KeepRelative" true))