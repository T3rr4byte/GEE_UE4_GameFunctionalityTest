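; AI controller for the Zombie10 enemy that runs BT_Zombie10 when it possesses the zombie.
; AI perception of the player writes CanSeePlayer to the blackboard; on lost sight it stores the player's current location and sets RecentlySighted.
; Walk, Run and Attack events forward to the pawn, and Tick stops the brain logic once the zombie is dead.
; An unconnected block for saving a home location never runs.
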(event `self.ReceiveTick`
  (params (DeltaSeconds :type "Float (single-precision)"))
  ;[1 1 1] Death
  (bind _asbp_zombie_10 (cast `/Game/ThirdPersonBP/Blueprints/BP_Zombie10` (`self.Zombie10`)))
  (if (`/Game/ThirdPersonBP/Blueprints/BP_Zombie10.isDead?` _asbp_zombie_10)
    (`BrainComponent.StopLogic` (`AIController.BrainComponent` (`AIBlueprintHelperLibrary.GetAIController` self)) "Dead")))

(event `self.AIPerception.OnTargetPerceptionUpdated`
  (params (Actor :type "Actor Object Reference") (Stimulus :type "AIStimulus Structure"))
  (bind (_age _expirationage _strength _stimuluslocation _receiverlocation _tag _bsuccessfullysensed) (break `AIStimulus` Stimulus))
  (bind _returnvalue (`AIBlueprintHelperLibrary.GetBlackboard` null))
  (cast `/Game/ThirdPersonBP/Blueprints/ThirdPersonCharacter` Actor)
  (`BlackboardComponent.SetValueAsBool` _returnvalue "CanSeePlayer" _bsuccessfullysensed)
  (if (not _bsuccessfullysensed)
    (`BlackboardComponent.SetValueAsVector` _returnvalue "PlayerLocation" (`self.K2_GetActorLocation` (`GameplayStatics.GetPlayerCharacter` 0)))
    (`BlackboardComponent.SetValueAsBool` _returnvalue "RecentlySighted" true)))

(event `Walk`
  (`/Game/ThirdPersonBP/Blueprints/BP_Zombie10.Walk` (`self.Zombie10`)))

(event `Run`
  (`/Game/ThirdPersonBP/Blueprints/BP_Zombie10.Run` (`self.Zombie10`)))

(event `self.OnPossess`
  (params (PossessedPawn :type "Pawn Object Reference"))
  (bind _asbp_zombie_10 (cast `/Game/ThirdPersonBP/Blueprints/BP_Zombie10` PossessedPawn))
  (set `self.Zombie10` _asbp_zombie_10)
  (`self.RunBehaviorTree` "/Game/Enemy/Zombie10/BT_Zombie10.BT_Zombie10"))

(event `Attack`
  (`/Game/ThirdPersonBP/Blueprints/BP_Zombie10.Attack` (`self.Zombie10`)))

(fn `UserConstructionScript`)